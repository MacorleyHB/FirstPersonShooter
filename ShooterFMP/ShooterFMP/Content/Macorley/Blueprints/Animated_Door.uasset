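; Animated door Blueprint that slides open when a Character enters its trigger volume.
; BeginPlay caches the world locations of the StartPoint and EndPoint components.
; PlayerTouch overlap plays a timeline that lerps the Door component between those points with a swept move.
; The file has no end-overlap handling or reverse playback to close the door.
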(event OnComponentBeginOverlap(PlayerTouch)
  (params (OverlappedComponent :type Primitive%20Component%20Object%20Reference) (OtherActor :type Actor%20Object%20Reference) (OtherComp :type Primitive%20Component%20Object%20Reference) (OtherBodyIndex :type Integer) (bFromSweep :type Boolean) (SweepResult :type Hit%20Result%20Structure%20%28by%20ref%29))
  (Utilities|Casting|CastToCharacter OtherActor)
  (bind _newtrack_0 (Timeline|Timeline_0 Play)
    (:Update
      (Transformation|SetWorldLocation (Variables|Default|GetDoor) (Math|Vector|Lerp(Vector) (Variables|Default|GetStart_Loc) (Variables|Default|GetEnd_Loc) _newtrack_0) true false))))

(event EventBeginPlay
  (Variables|Default|SetStart_Loc (Transformation|GetWorldLocation (Variables|Default|GetStart_Point)))
  (Variables|Default|SetEnd_Loc (Transformation|GetWorldLocation (Variables|Default|GetEnd_Point))))

(fn ConstructionScript)