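; Sliding double door for the underground tunnel that opens automatically for the Character_Hero.
; Entering the Box trigger plays two timelines, DoorLeft and DoorRight, which drive the relative Y location of the Left and Right panels.
; Leaving the box reverses both timelines after a short delay to close the door.
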(event OnComponentBeginOverlap(Box)
  (params (OverlappedComponent :type Primitive%20Component%20Object%20Reference) (OtherActor :type Actor%20Object%20Reference) (OtherComp :type Primitive%20Component%20Object%20Reference) (OtherBodyIndex :type Integer) (bFromSweep :type Boolean) (SweepResult :type Hit%20Result%20Structure%20%28by%20ref%29))
  ;[1 1 1] Left Door
  (Utilities|Casting|CastToCharacter_Hero OtherActor)
  (Utilities|FlowControl|Sequence
    (:then_0
      (bind _left (Timeline|DoorLeft Play)
        (:Update
          (Transformation|SetRelativeLocation (Variables|Default|GetLeft) (Math|Vector|MakeVector 0.0 _left 0.0) false false))))
    (:then_1
      ;[1 1 1] Right Door
      (bind _right (Timeline|DoorRight Play)
        (:Update
          (Transformation|SetRelativeLocation (Variables|Default|GetRight) (Math|Vector|MakeVector 0.0 _right 0.0) false false))))))

(event OnComponentEndOverlap(Box)
  (params (OverlappedComponent :type Primitive%20Component%20Object%20Reference) (OtherActor :type Actor%20Object%20Reference) (OtherComp :type Primitive%20Component%20Object%20Reference) (OtherBodyIndex :type Integer))
  ;[1 1 1] Right Door
  (Utilities|Casting|CastToCharacter_Hero OtherActor)
  (Utilities|FlowControl|Sequence
    (:then_0
      (Utilities|FlowControl|Delay 1.0)
      ;[1 1 1] Left Door
      (bind _left (Timeline|DoorLeft Reverse)
        (:Update
          (Transformation|SetRelativeLocation (Variables|Default|GetLeft) (Math|Vector|MakeVector 0.0 _left 0.0) false false))))
    (:then_1
      (Utilities|FlowControl|Delay 1.0)
      (bind _right (Timeline|DoorRight Reverse)
        (:Update
          (Transformation|SetRelativeLocation (Variables|Default|GetRight) (Math|Vector|MakeVector 0.0 _right 0.0) false false))))))

(fn ConstructionScript)