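; Health pickup actor that restores the hero's health when touched.
; On sphere overlap with a Character_Hero, it adds the Heal amount to Health, clamped to MaxHealth, then plays a regeneration sound and destroys itself.
; A hero already at full health leaves the pickup in place.
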(event OnComponentBeginOverlap(Sphere1)
  (params (OverlappedComponent :type Primitive%20Component%20Object%20Reference) (OtherActor :type Actor%20Object%20Reference) (OtherComp :type Primitive%20Component%20Object%20Reference) (OtherBodyIndex :type Integer) (bFromSweep :type Boolean) (SweepResult :type Hit%20Result%20Structure%20%28by%20ref%29))
  (bind _ascharacter_hero (Utilities|Casting|CastToCharacter_Hero OtherActor))
  (bind _output_get (Variables|Default|SetPlayer%20HP (Variables|/Game/Oli/Blueprints/Characters/Character_Hero.Character_Hero_C|GetHealth _ascharacter_hero)))
  (bind _output_get_2 (Variables|Default|SetPlayer%20Max%20HP (Variables|/Game/Oli/Blueprints/Characters/Character_Hero.Character_Hero_C|GetMaxHealth _ascharacter_hero)))
  (if (not (== (Variables|Default|GetPlayer%20HP) (Variables|Default|GetPlayer%20Max%20HP)))
    (if (> _output_get_2 (+ _output_get (Variables|Default|GetHeal)))
      (Variables|Default|SetHealing (+ _output_get (Variables|Default|GetHeal)))
      (else
        (Variables|Default|SetHealing (Variables|Default|GetPlayer%20Max%20HP))))
    (Variables|/Game/Oli/Blueprints/Characters/Character_Hero.Character_Hero_C|SetHealth _ascharacter_hero (Variables|Default|GetHealing))
    (Audio|PlaySound2D "/Game/Oli/Resources/Sounds/588251__romeo_kaleikau__power-up-regeneration-sfx.588251__romeo_kaleikau__power-up-regeneration-sfx" 1.0 1.0 0.0 0 0)
    (Actor|DestroyActor)))

(event EventBeginPlay)

(event Collision|EventActorBeginOverlap
  (params (OtherActor :type Actor%20Object%20Reference)))

(event EventTick
  (params (DeltaSeconds :type Float%20%28single-precision%29)))

(fn ConstructionScript)