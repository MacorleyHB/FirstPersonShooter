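; AggroZone is a trigger actor that aggroes nearby drones when the FPS character enters it.
; On BeginPlay it sizes its sphere to AggroRadius and draws a temporary debug sphere of that radius.
; The first character overlap, gated by a DoOnce, scans all DronePawn actors.
; Each drone within the radius of the zone gets the character as GoalActor and has its AggroEvent called.
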(event OnComponentBeginOverlap(Sphere)
  (params (OverlappedComponent :type Primitive%20Component%20Object%20Reference) (OtherActor :type Actor%20Object%20Reference) (OtherComp :type Primitive%20Component%20Object%20Reference) (OtherBodyIndex :type Integer) (bFromSweep :type Boolean) (SweepResult :type Hit%20Result%20Structure%20%28by%20ref%29))
  (bind _asfps_character (Utilities|Casting|CastToFPS_Character OtherActor))
  (Utilities|FlowControl|DoOnce false
    (:Completed
      (bind _outactors (Actor|GetAllActorsOfClass "/Game/Oli/Blueprints/Enemies/Drone/DronePawn.DronePawn_C"))
      (for _array_element _outactors
        (Variables|Default|SetCurrent%20Drone _array_element)
        (if (<= (Transformation|GetDistanceTo _array_element) (Variables|Default|GetAggro%20Radius))
          (Variables|/Game/Oli/Blueprints/Enemies/Drone/DronePawn.DronePawn_C|SetGoalActor (Variables|Default|GetCurrent%20Drone) _asfps_character)
          (Default|AggroEvent (Variables|Default|GetCurrent%20Drone)))))))

(event EventBeginPlay
  (Components|Sphere|SetSphereRadius (Variables|Default|GetSphere) (Variables|Default|GetAggro%20Radius) true)
  (Rendering|Debug|DrawDebugSphere (Transformation|GetActorLocation) (Variables|Default|GetAggro%20Radius) 24 "(R=1.000000,G=1.000000,B=1.000000,A=1.000000)" 6e+01 1.0))

(fn ConstructionScript)