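; Boss projectile that charges up by growing at its spawn point before it launches.
; On begin play, collision and velocity are off while a timeline scales it toward its final size, tracking the Spawn component's location and rotation.
; If Spawn becomes invalid during charging, it destroys itself.
; After a short delay, it applies its local velocity, enables query collision and only then runs the parent BeginPlay.
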(event EventBeginPlay
  (bind _spawn (Variables|Default|GetSpawn))
  (Collision|SetCollisionEnabled (Variables|Default|GetSphere1) "NoCollision")
  (Game|Components|ProjectileMovement|SetVelocityinLocalSpace (Variables|Default|GetProjectileMovement) "0, 0, 0")
  (bind _scale_line (Timeline|Scale%20Line PlayFromStart)
    (:Update
      (Utilities|IsValid _spawn
        (:Is%20Valid
          (Transformation|SetActorTransform (Math|Transform|MakeTransform (Transformation|GetWorldLocation _spawn) (Transformation|GetWorldRotation _spawn) (Math|Conversions|ToVector(Float) (* _scale_line (Variables|Default|GetFinal%20Scale))))))
        (:Is%20Not%20Valid
          (Actor|DestroyActor))))
    (:Finished
      (Utilities|FlowControl|Delay 0.3)
      (Game|Components|ProjectileMovement|SetVelocityinLocalSpace (Variables|Default|GetProjectileMovement) (Variables|Default|GetProjectile%20Velocity))
      (Collision|SetCollisionEnabled (Variables|Default|GetSphere1) "QueryOnly")
      (|CallParentFunction))))

(event Collision|EventActorBeginOverlap
  (params (OtherActor :type Actor%20Object%20Reference))
  (|CallParentFunction OtherActor) ; This node is disabled and will not be called.\nDrag off pins to build functionality.
)

(event EventTick
  (params (DeltaSeconds :type Float%20%28single-precision%29)))

(fn ConstructionScript
  (|CallParentFunction))