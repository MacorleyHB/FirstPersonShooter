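; Dummy is an enemy Blueprint that leaves most of its behavior to its parent class, adding only a small reaction to taking damage.
; On damage it runs the parent handler, then hides the ExposeWidget if the Exposed flag is false.
; A disconnected branch that would also call Explode at zero health never runs, and the construction script only calls the parent.
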(event EventBeginPlay
  (|CallParentFunction) ; This node is disabled and will not be called.\nDrag off pins to build functionality.
)

(event Collision|EventActorBeginOverlap
  (params (OtherActor :type Actor%20Object%20Reference)))

(event EventTick
  (params (DeltaSeconds :type Float%20%28single-precision%29))
  (|CallParentFunction DeltaSeconds) ; This node is disabled and will not be called.\nDrag off pins to build functionality.
)

(event EventOnTakeDamage
  (params (DamagedActor :type Actor%20Object%20Reference) (Damage :type Float%20%28single-precision%29) (DamageType :type Damage%20Type%20Object%20Reference) (InstigatedBy :type Controller%20Object%20Reference) (DamageCauser :type Actor%20Object%20Reference))
  (|CallParentFunction DamagedActor Damage DamageType InstigatedBy DamageCauser)
  (if (not (Variables|Default|GetExposed))
    (Rendering|SetVisibility (Variables|Default|GetExpose%20Widget) false false)))

(fn ConstructionScript
  (|CallParentFunction))