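; Flashbang projectile for the Sunslinger hero that acts as a rising, expanding burst rather than calling its parent BeginPlay.
; On spawn it caches the instigating hero, then a timeline lifts it from its start location while driving its scale, and destroys it when finished.
; Enemies overlapping the ImpactSphere are burned only if that hero has a specific perk.
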(event OnComponentBeginOverlap(ImpactSphere)
  (params (OverlappedComponent :type Primitive%20Component%20Object%20Reference) (OtherActor :type Actor%20Object%20Reference) (OtherComp :type Primitive%20Component%20Object%20Reference) (OtherBodyIndex :type Integer) (bFromSweep :type Boolean) (SweepResult :type Hit%20Result%20Structure%20%28by%20ref%29))
  (if (Utilities|Array|ContainsItem (Variables|/Game/Oli/Blueprints/Characters/Character_Hero.Character_Hero_C|GetPerks (Variables|Default|GetPlayer)) "NewEnumerator2")
    (bind _asenemy (Utilities|Casting|CastToEnemy OtherActor))
    (Default|Burn _asenemy)))

(event Collision|EventActorBeginOverlap
  (params (OtherActor :type Actor%20Object%20Reference)))

(event EventTick
  (params (DeltaSeconds :type Float%20%28single-precision%29)))

(event EventBeginPlay
  (bind _ascharacter_hero (Utilities|Casting|CastToCharacter_Hero (Variables|Default|GetInstigator)))
  (Variables|Default|SetPlayer _ascharacter_hero)
  (Variables|Default|SetStart%20Location (Transformation|GetActorLocation))
  (Transformation|SetActorScale3D "0.100000,0.100000,0.100000")
  (bind (_direction _expand _go_up) (Timeline|Expand%20Line PlayFromStart)
    (:Update
      (Transformation|SetActorLocation (Math|Vector|MakeVector (.x (Variables|Default|GetStart%20Location)) (.y (Variables|Default|GetStart%20Location)) (+ _go_up (.z (Variables|Default|GetStart%20Location)))) false false)
      (Transformation|SetActorScale3D (Math|Conversions|ToVector(Float) _expand)))
    (:Finished
      (Actor|DestroyActor))))

(fn ConstructionScript
  (|CallParentFunction))