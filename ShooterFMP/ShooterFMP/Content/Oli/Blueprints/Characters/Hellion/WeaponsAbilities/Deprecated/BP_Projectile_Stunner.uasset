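; Deprecated Hellion stunner projectile that stuns Drones instead of dealing damage.
; When Sphere1 overlaps any actor, it zeroes Damage and ExtraDamage, then casts the actor to Drone and sets IsStunned.
; BeginPlay also clears ExtraDamage, and the remaining projectile behavior is left to the parent class.
; Nothing in this Blueprint clears the stun.
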(event OnComponentBeginOverlap(Sphere1)
  (params (OverlappedComponent :type Primitive%20Component%20Object%20Reference) (OtherActor :type Actor%20Object%20Reference) (OtherComp :type Primitive%20Component%20Object%20Reference) (OtherBodyIndex :type Integer) (bFromSweep :type Boolean) (SweepResult :type Hit%20Result%20Structure%20%28by%20ref%29))
  (Variables|Default|SetExtraDamage 0.0)
  (Variables|Default|SetDamage 0.0)
  (bind _asdrone (Utilities|Casting|CastToDrone OtherActor))
  (Variables|/Game/Oli/Blueprints/Enemies/Enemy.Enemy_C|SetIsStunned _asdrone true))

(event EventBeginPlay
  (Variables|Default|SetExtraDamage 0.0)
  (|CallParentFunction))

(event Collision|EventActorBeginOverlap
  (params (OtherActor :type Actor%20Object%20Reference))
  (|CallParentFunction OtherActor))

(event EventTick
  (params (DeltaSeconds :type Float%20%28single-precision%29)))

(fn ConstructionScript
  (|CallParentFunction))