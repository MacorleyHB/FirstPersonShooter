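; FlytextBP is a floating damage text actor that shows a number rising from its spawn point.
; On BeginPlay it writes its Damage value into the Flytext user widget held by its Widget component.
; The UpLine timeline then raises the actor along Z from its start transform, scaled by UpMultiplier, and destroys it when finished.
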(event EventBeginPlay
  (bind _asflytext (Utilities|Casting|CastToFlytext (UserInterface|GetUserWidgetObject (Variables|Default|GetWidget))))
  (Rendering|Components|TextRender|SetText (Variables|/Game/Oli/Resources/Flytext.Flytext_C|GetDamageText _asflytext) (Utilities|Text|ToText(Float) (Variables|Default|GetDamage) "HalfToEven"))
  (Variables|Default|SetStart%20Position (Transformation|GetActorTransform))
  (bind _go_up (Timeline|Up%20Line Play)
    (:Update
      (Transformation|SetActorTransform (Math|Transform|MakeTransform (Math|Vector|MakeVector (.x (.location (Variables|Default|GetStart%20Position))) (.y (.location (Variables|Default|GetStart%20Position))) (+ (.z (.location (Variables|Default|GetStart%20Position))) (* _go_up (Variables|Default|GetUp%20Multiplier)))) (.rotation (Variables|Default|GetStart%20Position)) (.scale (Variables|Default|GetStart%20Position)))))
    (:Finished
      (Actor|DestroyActor))))

(event Collision|EventActorBeginOverlap
  (params (OtherActor :type Actor%20Object%20Reference)))

(event EventTick
  (params (DeltaSeconds :type Float%20%28single-precision%29)))

(fn ConstructionScript)